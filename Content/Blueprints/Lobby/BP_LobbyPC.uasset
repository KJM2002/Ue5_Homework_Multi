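; BP_LobbyPC is the lobby player controller that sets up the lobby screen for the local player.
; On BeginPlay, if locally controlled, it creates and stores WBP_Lobby, adds it to the viewport, shows the cursor and switches to Game and UI input.
; An authority check then calls the widget's ShowStartButton with false only on the host, as the Korean comment notes.
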(event EventBeginPlay
  ;[0.15 0.15 0.15 0.5] Show Lobby Widget
  (if (Pawn|IsLocalPlayerController)
    (bind _returnvalue (UserInterface|CreateWidget "/Game/Blueprints/Lobby/UI/WBP_Lobby.WBP_Lobby_C" self))
    (bind _output_get (Variables|Default|SetLobbyWidgetObject _returnvalue))
    (UserInterface|Viewport|AddtoViewport _output_get 0)
    (Variables|Default|SetbShowMouseCursor true)
    (Input|SetInputModeGameandUI self 0 "DoNotLock" true false)
    ;;[0.15 0.15 0.15 0.5] 방장일때만
    (Networking|SwitchHasAuthority
      (:Authority
        (Class|LobbyWidgetBase|ShowStartButton (Variables|Default|GetLobbyWidgetObject) false)))))

(fn ConstructionScript)